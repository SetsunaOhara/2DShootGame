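; BP_Rewards is a moving pickup whose reward type (EnumReward) selects its flipbook sprite and scale.
; On BeginPlay it picks a random direction from VelocityArray and drives ProjectileMovement at Speed.
; Sphere overlaps with "Wall" actors bounce it manually, flipping X for "LR" walls and Z for others.
; Overlapping a "P"-tagged actor passes the type through GetRewardMessage, then destroys the pickup.
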(event OnComponentBeginOverlap(Sphere)
  (params (OverlappedComponent :type Primitive%20Component%20Object%20Reference) (OtherActor :type Actor%20Object%20Reference) (OtherComp :type Primitive%20Component%20Object%20Reference) (OtherBodyIndex :type Integer) (bFromSweep :type Boolean) (SweepResult :type Hit%20Result%20Structure%20%28by%20ref%29))
  (if (Actor|ActorHasTag OtherActor "Wall")
    (if (Actor|ActorHasTag OtherActor "LR")
      (Variables|Default|SetCurVelocity (Math|Vector|MakeVector (* (.x (Variables|Default|GetCurVelocity)) -1.0) (.y (Variables|Default|GetCurVelocity)) (.z (Variables|Default|GetCurVelocity))))
      (else
        (Variables|Default|SetCurVelocity (Math|Vector|MakeVector (.x (Variables|Default|GetCurVelocity)) (.y (Variables|Default|GetCurVelocity)) (* (.z (Variables|Default|GetCurVelocity)) -1.0)))))
    (Game|Components|ProjectileMovement|SetVelocityinLocalSpace (Variables|Default|GetProjectileMovement) (* (Variables|Default|GetCurVelocity) (Variables|Default|GetSpeed)))
    (elif (Actor|ActorHasTag OtherActor "P")
      (Class|IFPlayer|GetReward(Message) OtherActor (Variables|Default|GetEnum_Reward))
      (Actor|DestroyActor) ; 道具吃完之后就销毁
    )))

(event EventBeginPlay
  (bind _output_get (Variables|Default|SetCurVelocity (.OutItem (Utilities|Array|Random (Variables|Default|GetVelocityArray)))))
  (Game|Components|ProjectileMovement|SetVelocityinLocalSpace (Variables|Default|GetProjectileMovement) (* _output_get (Variables|Default|GetSpeed)))
  (Sprite|SetFlipbook (Variables|Default|GetPaperFlipbook) (Utilities|Select :Index (Variables|Default|GetEnum_Reward) :NewEnumerator0 "/Game/Rewards/HP/HP_capsule_FB.HP_capsule_FB" :NewEnumerator1 "/Game/Rewards/Bullet/B1_FB.B1_FB" :NewEnumerator2 "/Game/Rewards/Bullet/B2_FD.B2_FD" :NewEnumerator3 "/Game/Rewards/Bullet/B3_FD.B3_FD" :NewEnumerator4 0))
  (Transformation|SetRelativeScale3D (Variables|Default|GetPaperFlipbook) (Utilities|Select :Index (Variables|Default|GetEnum_Reward) :NewEnumerator0 "1.000000,1.000000,1.000000" :NewEnumerator1 "1.000000,1.000000,1.000000" :NewEnumerator2 "3.000000,3.000000,3.000000" :NewEnumerator3 "1.000000,1.000000,1.000000" :NewEnumerator4 "0, 0, 0")))

(event Collision|EventActorBeginOverlap
  (params (OtherActor :type Actor%20Object%20Reference)))

(event EventTick
  (params (DeltaSeconds :type Float%20%28single-precision%29)))

(fn ConstructionScript)