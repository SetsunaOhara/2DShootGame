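; Shared 2D flipbook enemy covering four types (E1–E4, E4 being a boss) that damage the player on contact.
; Init loads stats and idle animation from DT_Enemy by enum name, then starts type-specific movement.
; E1 follows a spline on Tick; others use runtime-added ProjectileMovement, with E2 and E4 pausing for randomized bullet bursts.
; Hits flash red; death awards score, spawns effects and drops collision, with a splash overlap destroying the actor.
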(event OnComponentBeginOverlap(CapsuleComponent)
  (params (OverlappedComponent :type Primitive%20Component%20Object%20Reference) (OtherActor :type Actor%20Object%20Reference) (OtherComp :type Primitive%20Component%20Object%20Reference) (OtherBodyIndex :type Integer) (bFromSweep :type Boolean) (SweepResult :type Hit%20Result%20Structure%20%28by%20ref%29))
  ;[1 1 1] 敌人掉进水里 和水重叠并产生水花特效
  (Game|SpawnActorfromClass "/Game/Player/BP_Effect.BP_Effect_C" (Math|Transform|MakeTransform (Transformation|GetActorLocation) "0, 0, 0" "0.600000,0.600000,0.600000") "Undefined" "MultiplyWithRoot" 0 "/Game/Effects/Splash_1/Splash_FB_1.Splash_FB_1" false "(R=1.000000,G=1.000000,B=1.000000,A=1.000000)" 1.0 0)
  (Utilities|FlowControl|Delay 0.2)
  (Actor|DestroyActor))

(event OnComponentBeginOverlap(Capsule)
  (params (OverlappedComponent :type Primitive%20Component%20Object%20Reference) (OtherActor :type Actor%20Object%20Reference) (OtherComp :type Primitive%20Component%20Object%20Reference) (OtherBodyIndex :type Integer) (bFromSweep :type Boolean) (SweepResult :type Hit%20Result%20Structure%20%28by%20ref%29))
  ;[1 1 1] 敌人和玩家重叠并使玩家受到伤害
  (Utilities|IsValid OtherActor
    (:Is%20Valid
      (if (Actor|ActorHasTag OtherActor "P")
        (Class|IFPlayer|DamagePlayer(Message) OtherActor (Variables|角色|GetATK))))))

(event Custom|E2
  ;[1 1 1] E2移动:给敌人添加发射物组件以实现飞行效果。飞行一段时间后停止在屏幕当中射击，然后走到屏幕右边，转身再继续射击，然后飞行离开屏幕
  ;;[1 1 1] 控制敌人往前走
  (bind _returnvalue (AddComponent|AddProjectileMovementComponent)) ; 给敌人添加发射物组件，通过发射物组件来控制敌人的速度
  (bind _output_get (Variables|Default|SetProjectile _returnvalue))
  (Variables|/Script/Engine.ProjectileMovementComponent|SetProjectileGravityScale _output_get 0.0)
  (Variables|/Script/Engine.MovementComponent|SetVelocity _output_get (select (Variables|Default|GetRight?) (Math|Vector|MakeVector (* (Variables|角色|GetSpeed) -1.0) 0.0 0.0) (Math|Vector|MakeVector (* (Variables|角色|GetSpeed) 1.0) 0.0 0.0)))
  (Utilities|FlowControl|Delay 1.7) ; 敌人持续移动3.5秒
  (Utilities|EnemyShoot) ; 控制地方朝着自身前方60度角随机范围内射出20枚子弹
  (Variables|/Script/Engine.MovementComponent|SetVelocity (Variables|Default|GetProjectile) (select (Variables|Default|GetRight?) (Math|Vector|MakeVector (* (Variables|角色|GetSpeed) -1.0) 0.0 0.0) (Math|Vector|MakeVector (* (Variables|角色|GetSpeed) 1.0) 0.0 0.0)))
  (Utilities|FlowControl|Delay 1.7)
  (Variables|Default|SetRight? (not (Variables|Default|GetRight?)))
  (Transformation|SetRelativeRotation (Variables|Default|GetSprite) "0.000000,180.000000,0.000000" false false)
  (Utilities|EnemyShoot)
  (Variables|/Script/Engine.MovementComponent|SetVelocity (Variables|Default|GetProjectile) (select (Variables|Default|GetRight?) (Math|Vector|MakeVector (* (Variables|角色|GetSpeed) -1.0) 0.0 0.0) (Math|Vector|MakeVector (* (Variables|角色|GetSpeed) 1.0) 0.0 0.0)))
  (Utilities|FlowControl|Delay 5.0))

(event Custom|HitFlash
  ;[1 1 1] 击中闪光效果
  (Sprite|SetSpriteColor (Variables|Default|GetSprite) "(R=1.000000,G=0.000000,B=0.000000,A=1.000000)")
  (Utilities|FlowControl|Delay 0.2)
  (Sprite|SetSpriteColor (Variables|Default|GetSprite) "(R=1.000000,G=1.000000,B=1.000000,A=1.000000)"))

(event Custom|E3
  ;[1 1 1] 控制敌人往前走
  (bind _returnvalue (AddComponent|AddProjectileMovementComponent)) ; 给敌人添加发射物组件，通过发射物组件来控制敌人的速度
  (bind _output_get (Variables|Default|SetProjectile _returnvalue))
  (Variables|/Script/Engine.ProjectileMovementComponent|SetProjectileGravityScale _output_get 0.0)
  (Variables|/Script/Engine.MovementComponent|SetVelocity _output_get (select (Variables|Default|GetRight?) (Math|Vector|MakeVector (* (Variables|角色|GetSpeed) -1.0) 0.0 0.0) (Math|Vector|MakeVector (* (Variables|角色|GetSpeed) 1.0) 0.0 0.0))))

(event Custom|E4
  ;[1 1 1] boss移动到屏幕右侧
  (bind _returnvalue (AddComponent|AddProjectileMovementComponent)) ; 给敌人添加发射物组件，通过发射物组件来控制敌人的速度
  (bind _output_get (Variables|Default|SetProjectile _returnvalue))
  (Variables|/Script/Engine.ProjectileMovementComponent|SetProjectileGravityScale _output_get 0.0)
  (Variables|/Script/Engine.MovementComponent|SetVelocity _output_get (select (Variables|Default|GetRight?) (Math|Vector|MakeVector (* (Variables|角色|GetSpeed) -1.0) 0.0 0.0) (Math|Vector|MakeVector (* (Variables|角色|GetSpeed) 1.0) 0.0 0.0)))
  (Utilities|FlowControl|Delay 1.8) ; 敌人持续移动1.8秒
  (Utilities|BossShoot)
  (Variables|/Script/Engine.MovementComponent|SetVelocity (Variables|Default|GetProjectile) (Math|Vector|MakeVector 0.0 0.0 (* (Variables|角色|GetSpeed) 1.0)))
  (Utilities|FlowControl|Delay 0.5) ; 敌人持续移动0.5秒
  (Utilities|BossShoot :!label _label)
  (Variables|/Script/Engine.MovementComponent|SetVelocity (Variables|Default|GetProjectile) (Math|Vector|MakeVector 0.0 0.0 (* (Variables|角色|GetSpeed) -1.0)))
  (Utilities|FlowControl|Delay 1.0) ; 敌人持续移动0.5秒
  (Utilities|BossShoot)
  (Variables|/Script/Engine.MovementComponent|SetVelocity (Variables|Default|GetProjectile) (Math|Vector|MakeVector 0.0 0.0 (* (Variables|角色|GetSpeed) 1.0)))
  (Utilities|FlowControl|Delay 1.0) ; 敌人持续移动0.5秒
  (goto _label))

(event EventBeginPlay
  ;[1 1 1] 初始化一些属性
  (Utilities|Init))

(event EventDamageEnemy
  (params (Damage :type Float%20%28double-precision%29) (BulletIndex :type Enum_PlayerBullet%20Enum :default "NewEnumerator0"))
  ;[1 1 1] 玩家伤害敌人
  (if (Variables|Default|GetcanDamage)
    (Utilities|UpdateHP Damage BulletIndex)))

(event EventTick
  (params (DeltaSeconds :type Float%20%28single-precision%29))
  ;[1 1 1] tick:沿着样条线移动
  (switch Utilities|FlowControl|Switch|SwitchonEnum_Enemy (Variables|Character|GetEnum_Enemy)
    (:NewEnumerator0
      (switch Utilities|FlowControl|Switch|SwitchonEnum_Action (Variables|Default|GetEnum_Action)
        (:NewEnumerator0
          _)
        (:NewEnumerator1
          _))
      (bind _output_get (Variables|Default|SetDistance (+ (* DeltaSeconds (Variables|角色|GetSpeed)) (Variables|Default|GetDistance))))
      (Transformation|SetActorLocation (.location (Spline|GetTransformatDistanceAlongSpline (Variables|Default|GetSpline) _output_get "World" false)) false false))))

(fn ConstructionScript)