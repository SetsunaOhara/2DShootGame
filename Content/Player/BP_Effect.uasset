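; BP_Effect is a Paper2D effect actor that plays a configurable flipbook animation.
; On BeginPlay it applies its flipbook, looping, color and play rate variables to the PaperFlipbook component.
; When the flipbook finishes playing and looping is off, the actor destroys itself, so one-shot effects clean up automatically.
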(event OnFinishedPlaying(PaperFlipbook)
  (if (not (Variables|Default|GetNew%20Looping))
    (Actor|DestroyActor)))

(event EventBeginPlay
  (bind _paperflipbook (Variables|Default|GetPaperFlipbook))
  (Sprite|SetFlipbook _paperflipbook (Variables|Default|GetNew%20Flipbook))
  (Components|Timeline|SetLooping _paperflipbook (Variables|Default|GetNew%20Looping))
  (Sprite|SetSpriteColor _paperflipbook (Variables|Default|GetNew%20Color))
  (Components|Timeline|SetPlayRate (Variables|Default|GetPaperFlipbook) (Variables|Default|GetNew%20Rate)))

(event Collision|EventActorBeginOverlap
  (params (OtherActor :type Actor%20Object%20Reference)))

(event EventTick
  (params (DeltaSeconds :type Float%20%28single-precision%29)))

(fn ConstructionScript)