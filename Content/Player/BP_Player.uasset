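; Player character for a 2D sprite shooter, with X/Z movement, flight animation states, rotatable wingmen and a HUD.
; Shooting fires both wingmen plus the selected bullet type, using per-level data and a fire-rate delay.
; Pickups add score, heal or unlock bullet types, which level up through hit experience.
; Damage triggers a red flash and timer-driven blinking invulnerability; zero HP disables input and collision and spawns a death effect.
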(event Custom|Hit%20Flash
  (Sprite|SetSpriteColor (Variables|Default|GetSprite) "(R=1.000000,G=0.000000,B=0.000000,A=1.000000)")
  (|PlayAnimationOverridewithCallbacks (Variables|Default|GetAs%20ABP%20Player) "/Game/Player/AnimSequences/Player_Hurt.Player_Hurt" "DefaultSlot" 1.0 0.0
    (:then
      (Utilities|FlowControl|Delay 0.2)
      (Sprite|SetSpriteColor (Variables|Default|GetSprite) "(R=1.000000,G=1.000000,B=1.000000,A=1.000000)"))))

(event Custom|Protect
  (bind _capsule (Variables|Default|GetCapsule))
  (Rendering|ToggleVisibility (Variables|Default|GetSprite) true)
  (bind _output_get (Variables|Default|SetProtectCount (+ 0.1 (Variables|Default|GetProtectCount))))
  (if (>= _output_get 1.5)
    (Variables|Default|SetProtectCount 0.0)
    (Utilities|Time|ClearandInvalidateTimerbyHandle (Variables|Default|GetProtectEffects_Handle))
    (Collision|SetCollisionResponsetoChannel _capsule "ECC_GameTraceChannel3" "ECR_Overlap")
    (Collision|SetCollisionResponsetoChannel _capsule "ECC_GameTraceChannel4" "ECR_Overlap")
    (Rendering|SetVisibility (Variables|Default|GetSprite) true true)))

(event Input|EnhancedActionEvents|EnhancedInputActionIA_1
  (params (ActionValue :type Boolean) (ElapsedSeconds :type Float%20%28double-precision%29) (TriggeredSeconds :type Float%20%28double-precision%29) (InputAction :type Input%20Action%20Object%20Reference :default "/Game/Input/IA_1.IA_1"))
  (:Started
    (Utilities|IFBulletActive "NewEnumerator0")))

(event Input|EnhancedActionEvents|EnhancedInputActionIA_2
  (params (ActionValue :type Boolean) (ElapsedSeconds :type Float%20%28double-precision%29) (TriggeredSeconds :type Float%20%28double-precision%29) (InputAction :type Input%20Action%20Object%20Reference :default "/Game/Input/IA_2.IA_2"))
  (:Started
    (Utilities|IFBulletActive "NewEnumerator1")))

(event Input|EnhancedActionEvents|EnhancedInputActionIA_3
  (params (ActionValue :type Boolean) (ElapsedSeconds :type Float%20%28double-precision%29) (TriggeredSeconds :type Float%20%28double-precision%29) (InputAction :type Input%20Action%20Object%20Reference :default "/Game/Input/IA_3.IA_3"))
  (:Started
    (Utilities|IFBulletActive "NewEnumerator2")))

(event Input|EnhancedActionEvents|EnhancedInputActionIA_E1
  (params (ActionValue :type Boolean) (ElapsedSeconds :type Float%20%28double-precision%29) (TriggeredSeconds :type Float%20%28double-precision%29) (InputAction :type Input%20Action%20Object%20Reference :default "/Game/Input/IA_E1.IA_E1")))

(event Input|EnhancedActionEvents|EnhancedInputActionIA_E2
  (params (ActionValue :type Boolean) (ElapsedSeconds :type Float%20%28double-precision%29) (TriggeredSeconds :type Float%20%28double-precision%29) (InputAction :type Input%20Action%20Object%20Reference :default "/Game/Input/IA_E2.IA_E2")))

(event Input|EnhancedActionEvents|EnhancedInputActionIA_E3
  (params (ActionValue :type Boolean) (ElapsedSeconds :type Float%20%28double-precision%29) (TriggeredSeconds :type Float%20%28double-precision%29) (InputAction :type Input%20Action%20Object%20Reference :default "/Game/Input/IA_E3.IA_E3")))

(event EventBeginPlay
  (Utilities|Init))

(event EventDamagePlayer
  (params (Damage :type Float%20%28double-precision%29))
  (Utilities|UpdateHp Damage))

(event EventGetReward
  (params (Reward :type Enum_Reward%20Enum :default "NewEnumerator0"))
  ;[1 1 1] 捡到物品加分
  (CallFunction|UpdateScore (Utilities|Select :Index Reward :NewEnumerator0 350 :NewEnumerator1 500 :NewEnumerator2 500 :NewEnumerator3 500 :NewEnumerator4 400))
  (switch Utilities|FlowControl|Switch|SwitchonEnum_Reward Reward
    (:NewEnumerator0
      (Utilities|UpdateHp -3.0) ; 加血
    )
    (:NewEnumerator1
      (CallFunction|ActiveBullet "NewEnumerator0"))
    (:NewEnumerator2
      (CallFunction|ActiveBullet "NewEnumerator1"))
    (:NewEnumerator3
      (CallFunction|ActiveBullet "NewEnumerator2"))))

(event EventUpdateUIScore
  (bind _ui_player (Variables|Default|GetUI_Player)
    (:then
      (Default|UpdateUIScore _ui_player))
    (:else)))

(event EventUpdateExpBullet
  (params (BulletIndex :type Enum_PlayerBullet%20Enum :default "NewEnumerator0"))
  ;[1 1 1] 子弹命中后增加经验值
  (CallFunction|UpdateBulletExpandLevel BulletIndex))

(event OnComponentBeginOverlap(Box)
  (params (OverlappedComponent :type Primitive%20Component%20Object%20Reference) (OtherActor :type Actor%20Object%20Reference) (OtherComp :type Primitive%20Component%20Object%20Reference) (OtherBodyIndex :type Integer) (bFromSweep :type Boolean) (SweepResult :type Hit%20Result%20Structure%20%28by%20ref%29))
  ;[1 1 1] Box overlap  与水面重叠溅起水花
  (if (Actor|ActorHasTag OtherActor "Water")
    (Development|SetHiddeninGame (Variables|Default|GetSplash) false false)))

(event OnComponentEndOverlap(Box)
  (params (OverlappedComponent :type Primitive%20Component%20Object%20Reference) (OtherActor :type Actor%20Object%20Reference) (OtherComp :type Primitive%20Component%20Object%20Reference) (OtherBodyIndex :type Integer))
  ;[1 1 1] Box overlap  与水面重叠溅起水花
  (Development|SetHiddeninGame (Variables|Default|GetSplash) true false))

(event Input|EnhancedActionEvents|EnhancedInputActionIA_Move
  (params (ActionValue :type Vector%202D%20Structure) (ElapsedSeconds :type Float%20%28double-precision%29) (TriggeredSeconds :type Float%20%28double-precision%29) (InputAction :type Input%20Action%20Object%20Reference :default "/Game/Input/IA_Move.IA_Move"))
  (bind (_x _y) (Math|Vector2D|BreakVector2D ActionValue))
  ;[1 1 1] 移动
  (:Triggered
    (Pawn|Input|AddMovementInput "1.000000,0.000000,0.000000" _x false)
    (Pawn|Input|AddMovementInput "0.000000,0.000000,1.000000" _y false)
    (if (== _y 1.0)
      (bind _output_get (Variables|Default|SetEnum_Fly "NewEnumerator1"))
      (Variables|/Game/Player/ABP_Player.ABP_Player_C|SetEnum_Fly (Variables|Default|GetAs%20ABP%20Player) _output_get)
      (elif (== _y -1.0)
        (bind _output_get_2 (Variables|Default|SetEnum_Fly "NewEnumerator2"))
        (Variables|/Game/Player/ABP_Player.ABP_Player_C|SetEnum_Fly (Variables|Default|GetAs%20ABP%20Player) _output_get_2)
        (else
          (bind _output_get_3 (Variables|Default|SetEnum_Fly "NewEnumerator0"))
          (Variables|/Game/Player/ABP_Player.ABP_Player_C|SetEnum_Fly (Variables|Default|GetAs%20ABP%20Player) _output_get_3)))))
  (:Completed
    (bind _output_get_4 (Variables|Default|SetEnum_Fly "NewEnumerator0"))
    (Variables|/Game/Player/ABP_Player.ABP_Player_C|SetEnum_Fly (Variables|Default|GetAs%20ABP%20Player) _output_get_4)))

(event Input|EnhancedActionEvents|EnhancedInputActionIA_Shoot
  (params (ActionValue :type Boolean) (ElapsedSeconds :type Float%20%28double-precision%29) (TriggeredSeconds :type Float%20%28double-precision%29) (InputAction :type Input%20Action%20Object%20Reference :default "/Game/Input/IA_Shoot.IA_Shoot"))
  (bind (_atk _velocity _life _bulletclass _bulletnum _bulletscale _destroy_) (Utilities|GetBulletData))
  (bind _shootpoint (Variables|Default|GetShootPoint))
  (bind _returnvalue (Transformation|GetWorldRotation _shootpoint))
  ;[1 1 1] 射击
  (switch Utilities|FlowControl|Switch|SwitchonEnum_Action (Variables|Default|GetEnum_Action)
    (:NewEnumerator0
      (for _index (range 0 1)
        ;;[1 1 1] 僚机射击
        (Game|SpawnActorfromClass "/Game/Player/BP_Player_Bullet_1.BP_Player_Bullet_1_C" (Math|Transform|MakeTransform (Utilities|Select :Index _index :Option%200 (Transformation|GetWorldLocation (Variables|Default|GetShootPoint1)) :Option%201 (Transformation|GetWorldLocation (Variables|Default|GetShootPoint2))) (Utilities|Select :Index _index :Option%200 (Transformation|GetWorldRotation (Variables|Default|GetShootPoint1)) :Option%201 (Transformation|GetWorldRotation (Variables|Default|GetShootPoint2))) "1.000000,1.000000,1.000000") "Undefined" "MultiplyWithRoot" 0 "1000.000000,0.000000,0.000000" (Variables|Default|GetATK) 1e+01 "NewEnumerator3" true 0))
      (for _index_2 (range 0 _bulletnum)
        (bind _output_get (Variables|Default|SetBullet _bulletclass))
        (Game|SpawnActorfromClass _output_get (Math|Transform|MakeTransform (Transformation|GetWorldLocation _shootpoint) (Math|Rotator|MakeRotator (.roll _returnvalue) (+ (.pitch _returnvalue) (Utilities|Array|Get(acopy) (Variables|Default|GetShootAngle) _index_2)) (.yaw _returnvalue)) _bulletscale) "Undefined" "MultiplyWithRoot" 0 _velocity _atk _life (Variables|Default|GetPlayerBullet) _destroy_ 0)
        (Variables|Default|SetEnum_Action "NewEnumerator1")
        (Utilities|FlowControl|Delay (Variables|Default|GetShootRate))
        (Variables|Default|SetEnum_Action "NewEnumerator0")))))

(event Input|EnhancedActionEvents|EnhancedInputActionIA_WL
  (params (ActionValue :type Boolean) (ElapsedSeconds :type Float%20%28double-precision%29) (TriggeredSeconds :type Float%20%28double-precision%29) (InputAction :type Input%20Action%20Object%20Reference :default "/Game/Input/IA_WL.IA_WL"))
  ;[1 1 1] 射击
  ;;[1 1 1] 僚机旋转
  (:Started
    (bind _新建轨道_0 (Timeline|Wingman%20Rotate Play)
      (:Update
        (Transformation|SetRelativeRotation (Variables|Default|GetWingman_1) (Math|Rotator|Lerp(Rotator) "0, 0, 0" "180.000000,0.000000,0.000000" _新建轨道_0) false false)
        (Transformation|SetRelativeRotation (Variables|Default|GetWingman_2) (Math|Rotator|Lerp(Rotator) "0, 0, 0" "-180.000000,0.000000,0.000000" _新建轨道_0) false false))))
  (:Completed
    (Timeline|Wingman%20Rotate Stop)))

(event Input|EnhancedActionEvents|EnhancedInputActionIA_WR
  (params (ActionValue :type Boolean) (ElapsedSeconds :type Float%20%28double-precision%29) (TriggeredSeconds :type Float%20%28double-precision%29) (InputAction :type Input%20Action%20Object%20Reference :default "/Game/Input/IA_WR.IA_WR"))
  ;[1 1 1] 射击
  ;;[1 1 1] 僚机旋转
  (:Triggered
    (bind _新建轨道_0 (Timeline|Wingman%20Rotate Reverse)
      (:Update
        (Transformation|SetRelativeRotation (Variables|Default|GetWingman_1) (Math|Rotator|Lerp(Rotator) "0, 0, 0" "180.000000,0.000000,0.000000" _新建轨道_0) false false)
        (Transformation|SetRelativeRotation (Variables|Default|GetWingman_2) (Math|Rotator|Lerp(Rotator) "0, 0, 0" "-180.000000,0.000000,0.000000" _新建轨道_0) false false))))
  (:Completed
    (Timeline|Wingman%20Rotate Stop)))

(fn ConstructionScript)

(fn UpdateUIHp
  (bind _ui_player (Variables|Default|GetUI_Player)
    (:then
      (Default|UpdateUIHp _ui_player (/ (Variables|Default|GetHP) (Variables|Default|GetHPMax))))
    (:else)))

(fn ActiveBullet
  (params (bullet :type Enum_PlayerBullet%20Enum :default "NewEnumerator0"))
  (if (not (.ReturnValue (Utilities|Map|Find (Variables|Default|GetPlayerBulletLevel) bullet)))
    ;[1 1 1] 捡到子弹发现对应子弹未激活，则子弹等级+1，并将其激活
    (Utilities|Map|Add (Variables|Default|GetPlayerBulletLevel) bullet 1)
    (bind _ui_player (Variables|Default|GetUI_Player)
      (:then
        (Default|ActiveBullet _ui_player bullet))
      (:else))))

(fn UpdateBulletExpandLevel
  (params (BulletIndex :type Enum_PlayerBullet%20Enum :default "NewEnumerator0"))
  (bind _playerbulletlevel (Variables|Default|GetPlayerBulletLevel))
  (bind _bulletexp (Variables|Default|GetBulletExp))
  (bind _playerbulletexp (Variables|Default|GetPlayerBulletExp))
  (bind _playerbulletlevel_2 (Variables|Default|GetPlayerBulletLevel))
  (bind _ui_player (Variables|Default|GetUI_Player))
  (bind _value (Utilities|Map|Find _playerbulletexp BulletIndex))
  (bind (_value_2 _returnvalue) (Utilities|Map|Find _playerbulletlevel BulletIndex))
  (bind _value_3 (Utilities|Map|Find _playerbulletlevel_2 BulletIndex))
  (bind _returnvalue_2 (+ _value _bulletexp))
  ;[1 1 1] 判断子弹是否存在，是否达到子弹最大等级
  (if _returnvalue
    (if (not (== _value_2 (Variables|Default|GetBulletLevelMax)))
      ;[1 1 1] 子弹存在且没有超过最大等级，+经验并更新UI
      (Utilities|Map|Add (Variables|Default|GetPlayerBulletExp) BulletIndex _returnvalue_2) ; 覆盖子弹的经验值map
      (Default|UpdateUIBulletExp (Variables|Default|GetUI_Player) BulletIndex (/ (Math|Conversions|ToFloat(Integer) _returnvalue_2) (Math|Conversions|ToFloat(Integer) (Variables|Default|GetBulletLevelUpExp))))
      ;[1 1 1] 判断加完经验之后是否可以升级
      (if (>= _returnvalue_2 (Variables|Default|GetBulletLevelUpExp))
        ;[1 1 1] 经验值超过最大值，可以升级，等级+1，经验清零
        (Utilities|Map|Add (Variables|Default|GetPlayerBulletExp) BulletIndex 0) ; 经验条满，更新ExpMap经验值为0
        (Default|UpdateUIBulletExp _ui_player BulletIndex 0.0) ; 更新UI界面的经验条
        (bind _result (Math|Integer|IncrementInt _value_3)
          (:%20%20
            (Utilities|Map|Add _playerbulletlevel_2 BulletIndex _result) ; 经验满了，等级+1，更新LevelMap
            (Default|UpdateUIBulletLevel _ui_player BulletIndex (/ (Math|Conversions|ToFloat(Integer) _value_3) (Math|Conversions|ToFloat(Integer) (Variables|Default|GetBulletLevelMax)))) ; 更新UI界面的等级
          ))))))